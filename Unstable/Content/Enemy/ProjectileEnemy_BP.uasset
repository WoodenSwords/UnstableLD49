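; Ranged enemy character that shoots projectiles at the player when its attack event fires.
; BeginPlay registers the enemy in its AI controller's blackboard as ProjectileEnemy, without calling the parent BeginPlay.
; AttackEvent plays a shooting animation and spawns a scaled projectile ahead of it, facing the player, with velocity set to the unit direction toward them.
; The projectile receives the enemy's damage settings, and the looping run animation resumes after a short delay.
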(event EventBeginPlay
  (bind _asenemy_aicontroller (Utilities|Casting|CastToEnemy_AIController (Pawn|GetController)))
  (AI|Components|Blackboard|SetValueasObject (AI|GetBlackboard _asenemy_aicontroller) (Utilities|Name|MakeLiteralName "ProjectileEnemy") self))

(event EventAttackEvent
  (bind _returnvalue (Transformation|GetActorTransform))
  (bind (_location _rotation _scale) (Math|Transform|BreakTransform _returnvalue))
  (Components|Animation|PlayAnimation (Variables|Character|GetMesh) "/Game/Shooting_Anim.Shooting_Anim" false)
  (bind _returnvalue_2 (Game|SpawnActorfromClass "/Game/Enemy/Projectile_BP.Projectile_BP_C" (Math|Transform|MakeTransform (+ _location (* (Transformation|GetActorForwardVector) (Math|Float|MakeLiteralFloat 45.0)) "0,0,100.000000") (Math|Rotator|FindLookatRotation _location (Transformation|GetActorLocation (Game|Player|GetPlayerPawn 0))) (* _scale "0.100000,0.100000,0.500000")) "Undefined" 0 0))
  (Variables|/Script/Engine.MovementComponent|SetVelocity (Actor|GetComponentbyClass _returnvalue_2 "/Script/Engine.ProjectileMovementComponent") (Math|Vector|Normalize (- (Transformation|GetActorLocation (Game|Player|GetPlayerPawn 0)) (Transformation|GetWorldLocation (Variables|Default|GetCapsuleComponent)))))
  (Variables|/Game/Enemy/Projectile_BP.Projectile_BP_C|SetDamageType _returnvalue_2 (Variables|Default|GetDamageType))
  (Variables|/Game/Enemy/Projectile_BP.Projectile_BP_C|SetDamage _returnvalue_2 (Variables|Default|GetDamageVal))
  (Utilities|FlowControl|Delay 1.0)
  (Components|Animation|PlayAnimation (Variables|Character|GetMesh) "/Game/Treadmill_Running_Anim.Treadmill_Running_Anim" true))

(fn ConstructionScript
  (|CallParentFunction))