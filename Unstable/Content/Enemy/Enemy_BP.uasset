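; Enemy character Blueprint that attacks the player, reacts to a run event and dies on any damage.
; BeginPlay seeds blackboard bools and binds dispatchers: Attack damages the player pawn, Run flags PlayerExploding and clears the player key.
; Damage disables capsule collision, ragdolls the mesh, clears the player key and unpossesses the AI controller.
; Tick starts a looping run animation once; its always-true speed check leaves the shooting-animation branch unreachable.
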(event Custom|Attack_Event
  ;[1 1 1] Attack player event
  (Game|Damage|ApplyDamage (Pawn|GetControlledPawn (Game|GetPlayerController 0)) (Variables|DamageStats|GetDamageVal) 0 0 (Variables|DamageStats|GetDamageType)))

(event Custom|Run_Event
  (bind _returnvalue (Pawn|GetController))
  (bind _returnvalue_2 (AI|GetBlackboard _returnvalue))
  (AI|Components|Blackboard|SetValueasBool _returnvalue_2 (Utilities|Name|MakeLiteralName "PlayerExploding") true)
  (AI|Components|Blackboard|SetValueasObject _returnvalue_2 (Utilities|Name|MakeLiteralName "Player_ObjKey") 0))

(event EventTick
  (params (DeltaSeconds :type Float%20%28single-precision%29))
  (if (>= (Math|Vector|VectorLength (Variables|/Script/Engine.MovementComponent|GetVelocity (Variables|Character|GetCharacterMovement))) 0.0)
    (Utilities|FlowControl|DoOnce false :!label _label
      (:Completed
        (Components|Animation|PlayAnimation (Variables|Character|GetMesh) "/Game/Treadmill_Running_Anim.Treadmill_Running_Anim" true)))
    (else
      (Components|Animation|SetAnimation (Variables|Character|GetMesh) "/Game/Shooting_Anim.Shooting_Anim")
      (goto _label Reset))))

(event Game|Damage|EventAnyDamage
  (params (Damage :type Float%20%28single-precision%29) (DamageType :type Damage%20Type%20Object%20Reference) (InstigatedBy :type Controller%20Object%20Reference) (DamageCauser :type Actor%20Object%20Reference))
  (bind _returnvalue (Pawn|GetController))
  ;[1 1 1] Damaged, death event
  (Collision|SetCollisionEnabled (Variables|Collision|GetCapsuleComponent) "NoCollision")
  (AI|Components|Blackboard|SetValueasObject (AI|GetBlackboard _returnvalue) (Utilities|Name|MakeLiteralName "Player_ObjKey") 0)
  (Physics|SetSimulatePhysics (Variables|Character|GetMesh) true)
  (Utilities|Casting|CastToAIController _returnvalue)
  (Pawn|UnPossess _returnvalue))

(event EventBeginPlay
  (bind _returnvalue (Pawn|GetController))
  (bind _returnvalue_2 (AI|GetBlackboard _returnvalue))
  ;[1 1 1] begin play
  (Utilities|FlowControl|Sequence
    (:then_0
      ;[1 1 1] Attack player event
      (EventDispatchers|BindEventtoAttack (delegate Custom|Attack_Event))
      (EventDispatchers|BindEventtoRun (delegate Custom|Run_Event)))
    (:then_1
      (AI|Components|Blackboard|SetValueasBool _returnvalue_2 (Utilities|Name|MakeLiteralName "True") true)
      (AI|Components|Blackboard|SetValueasBool _returnvalue_2 (Utilities|Name|MakeLiteralName "False") false))))

(fn ConstructionScript)